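; Player controller for a top-down camera game with building placement, showing the cursor and creating the main HUD on begin play.
; Movement, speed modifier, zoom, reset and mouse edge-scroll inputs drive the camera pawn's movement component, with a gate enabling mouse panning while Pan is held and edge scroll is disabled.
; It relays date and game-speed display updates to the HUD, forwards speed changes to the GameState, and previews a Barracks on B.
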(event `Key|B`
  (params (Key :type "Key Structure"))
  (:`Pressed`
    (`/Game/Core/Buildings/BP_BuildingManager.SetPreview` (`self.BuildingManager`) "Barracks")))

(event `self.ReceiveBeginPlay`
  (`|ExecutionSequence`
    (:`then_0`
      (set `self.bShowMouseCursor` true)
      (bind _asbp_camera_pawn (cast `/Game/Core/Player/BP_cameraPawn` (`GameplayStatics.GetPlayerPawn` 0)))
      (bind _output_get (set `self.CameraPawnRef` _asbp_camera_pawn))
      (set `self.CameraMovementRef` (`/Game/Core/Player/BP_cameraPawn.PawnMovementComponent` _output_get)))
    (:`then_1`
      (bind _returnvalue (`|CreateWidget` "/Game/Core/Widgets/WBP_MainUI.WBP_MainUI_C" self))
      (bind _output_get_2 (set `self.MainWidgetRef` _returnvalue))
      (`UserWidget.AddToViewport` _output_get_2 0)
      (`WidgetBlueprintLibrary.SetInputMode_GameAndUIEx` self _output_get_2 "LockInFullscreen"))))

(event `InputAxis|MoveForward`
  (params (AxisValue :type "Float (single-precision)"))
  (`/Game/Core/Player/BP_PawnMovementComponent.BasicMovementControls` (`self.CameraMovementRef`) AxisValue (stale `InputAxis|MoveRight` AxisValue) :!label _label))

(event `InputAxis|MoveRight`
  (params (AxisValue :type "Float (single-precision)"))
  (goto _label))

(event `InputAction|SpeedModifire`
  (params (Key :type "Key Structure"))
  (bind _cameramovementref (`self.CameraMovementRef`))
  (:`Pressed`
    (`/Game/Core/Player/BP_PawnMovementComponent.SetSpeedModifier` _cameramovementref 2.0))
  (:`Released`
    (`/Game/Core/Player/BP_PawnMovementComponent.SetSpeedModifier` _cameramovementref 1.0)))

(event `/Game/Core/Interfaces/BPI_GameTime.Set DateTime`
  (params (DateTimeStruct :type "DateTime Structure"))
  (message `/Game/Core/Interfaces/BPI_GameTime.Set DateTime` (`self.MainWidgetRef`) DateTimeStruct))

(event `/Game/Core/Interfaces/BPI_GameTime.UpdateGameSpeed`
  (params (NewSpeedMultiplier :type "Float (double-precision)"))
  (message `/Game/Core/Interfaces/BPI_GameTime.UpdateGameSpeed` (`GameplayStatics.GetGameState`) NewSpeedMultiplier))

(event `InputAxisKey|MouseX` :paused true
  (params (AxisValue :type "Float (single-precision)"))
  (`/Game/Core/Player/BP_PawnMovementComponent.EdgeScroll` (`self.CameraMovementRef`) :!label _label_2))

(event `/Game/Core/Interfaces/BPI_GameTime.SetGameSpeedInt`
  (params (GameSpeed :type "Float (double-precision)"))
  (message `/Game/Core/Interfaces/BPI_GameTime.SetGameSpeedInt` (`self.MainWidgetRef`) GameSpeed))

(event `InputAxisKey|MouseY` :paused true
  (params (AxisValue :type "Float (single-precision)"))
  (goto _label_2))

(event `InputAction|ZoomIn`
  (params (Key :type "Key Structure"))
  (:`Pressed`
    (`/Game/Core/Player/BP_PawnMovementComponent.ZoomIn` (`self.CameraMovementRef`))))

(event `InputAction|ZoomOut`
  (params (Key :type "Key Structure"))
  (:`Pressed`
    (`/Game/Core/Player/BP_PawnMovementComponent.ZoomOut` (`self.CameraMovementRef`))))

(event `InputAction|ZoomReset`
  (params (Key :type "Key Structure"))
  (:`Pressed`
    (`/Game/Core/Player/BP_PawnMovementComponent.ResetZoom` (`self.CameraMovementRef`))))

(event `InputAxisKey|MouseX` :paused true
  (params (AxisValue :type "Float (single-precision)"))
  (`/Engine/EditorBlueprintResources/StandardMacros.Gate` true :!label _label_3
    (:`Exit`
      (`/Game/Core/Player/BP_PawnMovementComponent.PanCamera` (`self.CameraMovementRef`) (* AxisValue (`self.PanSensitivity`))))))

(event `InputAction|Pan`
  (params (Key :type "Key Structure"))
  (bind _cameramovementref (`self.CameraMovementRef`))
  (:`Pressed`
    (`/Game/Core/Player/BP_PawnMovementComponent.SetDisableEdgeScroll` _cameramovementref true)
    (goto _label_3 :!via `Open`))
  (:`Released`
    (`/Game/Core/Player/BP_PawnMovementComponent.SetDisableEdgeScroll` _cameramovementref false)
    (goto _label_3 :!via `Close`)))

(event `InputAction|PanReset`
  (params (Key :type "Key Structure"))
  (:`Pressed`
    (`/Game/Core/Player/BP_PawnMovementComponent.ResetPan` (`self.CameraMovementRef`))))

(event `InputAction|ResetCamera`
  (params (Key :type "Key Structure"))
  (:`Pressed`
    (`/Game/Core/Player/BP_PawnMovementComponent.ResetCamera` (`self.CameraMovementRef`))))

(fn `UserConstructionScript`)